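; AI controller that sends its possessed AICharacter toward path nodes linked through NextNode references.
; BeginPlay caches the pawn and starts a move to its DesiredNode.
; Tick polls the move status and, whenever it differs from DesiredStatus, requests a move to the DesiredNode's NextNode.
; DesiredNode is only reassigned to itself, so this graph never advances it along the chain.
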(event `self.ReceiveBeginPlay`
  (bind _asaicharacter (cast `/Game/Blueprints/AIBehaviors/AICharacter` (`self.K2_GetPawn`)))
  (bind _output_get (set `self.Stored Pawn` _asaicharacter))
  (`self.MoveToActor` (`/Game/Blueprints/AIBehaviors/AICharacter.DesiredNode` _output_get) 20.0))

(event `self.ReceiveTick`
  (params (DeltaSeconds :type "Float (single-precision)"))
  (bind _stored_pawn (`self.Stored Pawn`))
  (bind _desirednode (`/Game/Blueprints/AIBehaviors/AICharacter.DesiredNode` _stored_pawn))
  (if (!= (`self.GetMoveStatus`) (`self.DesiredStatus`))
    (set `/Game/Blueprints/AIBehaviors/AICharacter.DesiredNode` _desirednode _stored_pawn)
    (`self.MoveToActor` (`/Game/Blueprints/AIBehaviors/PathNode.NextNode` _desirednode))))

(fn `UserConstructionScript`)